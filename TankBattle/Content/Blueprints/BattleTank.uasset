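; BattleTank is the tank Blueprint that translates player input into aiming, movement and firing.
; BeginPlay hands the barrel and turret to InitialiseComponentData and both tracks to the TankMovement component.
; Mouse axes drive controller yaw and inverted pitch, while forward and separate left/right turn axes forward to TankMovement handlers.
; The Fire action calls FireProjectile, so the graph only wires components and input, leaving the logic to the functions it calls.
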(event EventBeginPlay
  (Class|Tank|InitialiseComponentData (Variables|Default|GetBarrel) (Variables|Default|GetTurret))
  (Class|TankMovementComponent|Initialise (Variables|Default|GetTankMovement) (Variables|Default|GetLeftTrack) (Variables|Default|GetRightTrack)))

(event Input|ActionEvents|InputActionFire
  (params (Key :type Key%20Structure :default "None"))
  (:Pressed
    (Class|Tank|FireProjectile)))

(event Input|AxisEvents|InputAxisMoveForward
  (params (AxisValue :type Float%20%28single-precision%29))
  (Class|TankMovementComponent|HandleForwardMovement (Variables|Default|GetTankMovement) AxisValue))

(event Input|AxisEvents|InputAxisTurnRight
  (params (AxisValue :type Float%20%28single-precision%29))
  (Class|TankMovementComponent|HandleTurnRight (Variables|Default|GetTankMovement) AxisValue))

(event Input|AxisEvents|InputAxisTurnLeft
  (params (AxisValue :type Float%20%28single-precision%29))
  (Class|TankMovementComponent|HandleTurnLeft (Variables|Default|GetTankMovement) AxisValue))

(event Input|MouseEvents|MouseX
  (params (AxisValue :type Float%20%28single-precision%29))
  (Pawn|Input|AddControllerYawInput AxisValue))

(event Input|MouseEvents|MouseY
  (params (AxisValue :type Float%20%28single-precision%29))
  (Pawn|Input|AddControllerPitchInput (* AxisValue -1.0)))

(fn ConstructionScript)