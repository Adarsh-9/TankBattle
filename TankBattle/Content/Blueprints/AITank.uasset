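; AITank Blueprint for a tank with track movement, turret aiming, firing and a health bar.
; BeginPlay wires the tracks into TankMovement and the barrel and turret into TankAiming, and clamps the first player camera's view pitch.
; The Fire input action asks TankAiming to fire and plays a firing sound on success.
; Tick pushes the health percentage into the HealthBar widget; no AI logic appears in these graphs.
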(event EventBeginPlay
  (bind _returnvalue (Game|GetPlayerCameraManager 0))
  (Class|TankMovementComponent|Initialise (Variables|Default|GetTankMovement) (Variables|Default|GetTankTrackLeft) (Variables|Default|GetTankTrackRight))
  (Class|TankAimingComponent|Initialise (Variables|Default|GetTankAiming) (Variables|Default|GetBarrel) (Variables|Default|GetTurret))
  (Variables|/Script/Engine.PlayerCameraManager|SetViewPitchMax _returnvalue 15.0)
  (Variables|/Script/Engine.PlayerCameraManager|SetViewPitchMin _returnvalue -5.0))

(event Collision|EventActorBeginOverlap
  (params (OtherActor :type Actor%20Object%20Reference)))

(event EventTick
  (params (DeltaSeconds :type Float%20%28single-precision%29))
  (bind _ashealth_bar (Utilities|Casting|CastToHealthBar (UserInterface|GetUserWidgetObject (Variables|Default|GetHealthBar))))
  (Variables|/Game/UI/HealthBar.HealthBar_C|SetHealthPercentage _ashealth_bar (Class|Tank|GetHealthPercentage)))

(event EventOnDamageTakenEvent)

(event Input|ActionEvents|InputActionFire
  (params (Key :type Key%20Structure :default "None"))
  (:Pressed
    (bind _returnvalue (Class|TankAimingComponent|FireProjectile (Variables|Default|GetTankAiming)))
    (if _returnvalue
      (Audio|PlaySoundatLocation "/Game/SoundFX/TankFiring.TankFiring" (Transformation|GetActorLocation) "0, 0, 0" 1.0 1.0 0.0 0 0 0))))

(fn ConstructionScript)