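; Player-controlled tank pawn that drives, looks around, fires projectiles and shows its health.
; BeginPlay wires the tracks into TankMovement and the barrel and turret into TankAiming, then clamps camera pitch.
; Movement input goes to TankMovement and mouse input rotates the controller.
; A successful TankAiming shot triggers camera shake and sound, damage triggers its own shake, and Tick pushes health percentage to the HealthBar widget.
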(event EventBeginPlay
  (bind _returnvalue (Game|GetPlayerCameraManager 0))
  (Class|TankMovementComponent|Initialise (Variables|Default|GetTankMovement) (Variables|Default|GetTankTrackLeft) (Variables|Default|GetTankTrackRight))
  (Class|TankAimingComponent|Initialise (Variables|Default|GetTankAiming) (Variables|Default|GetBarrel) (Variables|Default|GetTurret))
  (Variables|/Script/Engine.PlayerCameraManager|SetViewPitchMax _returnvalue 15.0)
  (Variables|/Script/Engine.PlayerCameraManager|SetViewPitchMin _returnvalue -5.0))

(event Collision|EventActorBeginOverlap
  (params (OtherActor :type Actor%20Object%20Reference)))

(event EventTick
  (params (DeltaSeconds :type Float%20%28single-precision%29))
  (bind _ashealth_bar (Utilities|Casting|CastToHealthBar (UserInterface|GetUserWidgetObject (Variables|Default|GetHealthBar))))
  (Variables|/Game/UI/HealthBar.HealthBar_C|SetHealthPercentage _ashealth_bar (Class|Tank|GetHealthPercentage)))

(event EventOnDamageTakenEvent
  (Camera|PlayWorldCameraShake "/Game/Blueprints/DamageCameraShake.DamageCameraShake_C" (Transformation|GetActorLocation) 0.0 1.5e+03))

(event Input|ActionEvents|InputActionFire
  (params (Key :type Key%20Structure :default "None"))
  (bind _returnvalue (Transformation|GetActorLocation))
  (:Pressed
    (bind _returnvalue_2 (Class|TankAimingComponent|FireProjectile (Variables|Default|GetTankAiming)))
    (if _returnvalue_2
      (Camera|PlayWorldCameraShake "/Game/Blueprints/FireCameraShake.FireCameraShake_C" _returnvalue 0.0 1.5e+03)
      (Audio|PlaySoundatLocation "/Game/SoundFX/TankFiring.TankFiring" _returnvalue "0, 0, 0" 1.0 1.0 0.0 0 0 0))))

(event Input|AxisEvents|InputAxisMoveForward
  (params (AxisValue :type Float%20%28single-precision%29))
  (Class|TankMovementComponent|HandleForwardMovement (Variables|Default|GetTankMovement) AxisValue))

(event Input|AxisEvents|InputAxisTurnRight
  (params (AxisValue :type Float%20%28single-precision%29))
  (Class|TankMovementComponent|HandleTurnRight (Variables|Default|GetTankMovement) AxisValue))

(event Input|AxisEvents|InputAxisTurnLeft
  (params (AxisValue :type Float%20%28single-precision%29))
  (Class|TankMovementComponent|HandleTurnLeft (Variables|Default|GetTankMovement) AxisValue))

(event Input|MouseEvents|MouseX
  (params (AxisValue :type Float%20%28single-precision%29))
  (Pawn|Input|AddControllerYawInput AxisValue))

(event Input|MouseEvents|MouseY
  (params (AxisValue :type Float%20%28single-precision%29))
  (Pawn|Input|AddControllerPitchInput (* AxisValue -1.0)))

(fn ConstructionScript)