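; Player controller Blueprint for the tank that creates the player HUD and feeds it reload and health values.
; When the aiming component is found, it adds the PlayerUI widget to the viewport and passes it that component.
; Tick restarts a timeline whenever the status is not Reloading, so it only advances during a reload.
; Timeline updates write reload progress and the controlled tank's health percentage to the HUD.
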(event EventTick
  (params (DeltaSeconds :type Float%20%28single-precision%29))
  (bind _returnvalue (Class|TankPlayercontroller|GetControlledTank))
  (if (not (Utilities|Select :Index (Variables|/Script/TankBattle.TankAimingComponent|GetAimingStatus (Variables|Default|GetAimingComp)) :Reloading true :Aiming false :Locked false :OutOfAmmo false))
    (bind _progress (Timeline|Timeline_0 PlayFromStart)
      (:Update
        (Variables|/Game/UI/PlayerUI.PlayerUI_C|SetReloadProgress (Variables|Default|GetHUDRef) _progress)
        (Utilities|IsValid _returnvalue
          (:Is%20Valid
            (Variables|/Game/UI/PlayerUI.PlayerUI_C|SetHealthPercentage (Variables|Default|GetHUDRef) (Class|Tank|GetHealthPercentage (.AsPlayer%20Tank (Utilities|Casting|CastToPlayerTank _returnvalue))))))))))

(event EventFoundAimingcomponent
  (params (AimingComponentArg :type Tank%20Aiming%20Component%20Object%20Reference))
  (Variables|Default|SetAimingComp AimingComponentArg)
  (bind _returnvalue (UserInterface|CreateWidget "/Game/UI/PlayerUI.PlayerUI_C"))
  (bind _output_get (Variables|Default|SetHUDRef _returnvalue))
  (UserInterface|Viewport|AddtoViewport _output_get 0)
  (Variables|/Game/UI/PlayerUI.PlayerUI_C|SetAimComponentRef (Variables|Default|GetHUDRef) AimingComponentArg))

(fn ConstructionScript)